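; Wall_BP is a wall prop Blueprint built on a Cube component whose surface material is configurable.
; The construction script applies MaterialInstance to the Cube's first slot if valid, then applies Material to the same slot, so a valid Material takes precedence.
; The event graph holds only disabled placeholder events, so the wall adds no gameplay logic of its own.
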(event EventBeginPlay)

(event Collision|EventActorBeginOverlap
  (params (OtherActor :type Actor%20Object%20Reference)))

(event EventTick
  (params (DeltaSeconds :type Float%20%28single-precision%29)))

(fn ConstructionScript
  (Utilities|FlowControl|Sequence
    (:then_0
      (Utilities|IsValid (Variables|Default|GetMaterialInstance)
        (:Is%20Valid
          (Rendering|Material|SetMaterial (Variables|Default|GetCube) 0 (Variables|Default|GetMaterialInstance)))))
    (:then_1
      (Utilities|IsValid (Variables|Default|GetMaterial)
        (:Is%20Valid
          (Rendering|Material|SetMaterial (Variables|Default|GetCube) 0 (Variables|Default|GetMaterial)))))))