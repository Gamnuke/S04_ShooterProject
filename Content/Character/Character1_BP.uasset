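; Player character Blueprint that sets up a HUD, an aim point and a weapon component.
; BeginPlay creates the HUD widget for its player controller and adds it to that player's screen.
; Tick recomputes the aim point at horizontal centre, above mid-screen, from viewport size and prints it for debugging.
; The construction script hands the weapon mesh to the weapon component and stores the text render component.
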(event Collision|EventActorBeginOverlap
  (params (OtherActor :type Actor%20Object%20Reference)))

(event EventTick
  (params (DeltaSeconds :type Float%20%28single-precision%29))
  (bind _returnvalue (Viewport|GetViewportSize))
  (bind _output_get (Variables|Default|SetAimPointScreenLocation (Math|Vector2D|MakeVector2D (* (.x _returnvalue) 0.5) (* (.y _returnvalue) 0.3))))
  (Development|PrintString (Utilities|String|ToString(Vector2d) _output_get)))

(event EventBeginPlay
  (bind _asplayer_controller (Utilities|Casting|CastToPlayerController (Pawn|GetController)))
  (bind _returnvalue (UserInterface|CreateWidget "/Game/Character/HUD_BP.HUD_BP_C" _asplayer_controller))
  (UserInterface|Viewport|AddtoPlayerScreen _returnvalue))

(fn ConstructionScript
  (Variables|Default|SetTextRenderer (Variables|Default|GetTextRender))
  (Variables|/Script/ShooterProject.WeaponComponent|SetWeaponMesh (Variables|Default|GetWeaponComponent) (Variables|Default|GetWeaponMesh)))