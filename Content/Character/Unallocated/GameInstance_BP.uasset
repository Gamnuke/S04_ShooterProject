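; Game instance that handles front-end menu navigation and online session hosting.
; Events create and show the main, join, host, loading and lobby widgets with the mouse cursor enabled.
; CreateLobby creates a session with hardcoded settings, then on success swaps to the loading screen and calls SpawnCharacter, which only opens TestLevel.
; DestroySession ends the session, LogToScreen prints status, and character spawn/possess nodes are left unconnected.
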(event Custom|ToHostLobbyPlayersScreen
  (bind _returnvalue (Game|GetPlayerController 0))
  ;[1 1 1] Lobby screen
  (bind _returnvalue_2 (UserInterface|CreateWidget "/Game/Character/HUD/LobbyPlayers_WBP.LobbyPlayers_WBP_C" _returnvalue))
  (UserInterface|Viewport|AddtoPlayerScreen _returnvalue_2)
  (Variables|/Script/Engine.PlayerController|SetbShowMouseCursor _returnvalue true))

(event Custom|ToMainMenuScreen
  (bind _returnvalue (Game|GetPlayerController 0))
  ;[1 1 1] Main Menu Screen
  (bind _returnvalue_2 (UserInterface|CreateWidget "/Game/Character/HUD/MainMenu_B.MainMenu_B_C" _returnvalue))
  (UserInterface|Viewport|AddtoPlayerScreen _returnvalue_2)
  (Variables|/Script/Engine.PlayerController|SetbShowMouseCursor _returnvalue true)
  (Utilities|LogtoScreen "Made Main Menu"))

(event Custom|DestroySession
  ;[1 1 1] Create A Game Session
  (|DestroySession (Game|GetPlayerController 0)))

(event Custom|SpawnCharacter
  (params (PlayerController :type Player%20Controller%20Object%20Reference))
  (Game|OpenLevel(byName) "TestLevel"))

(event Custom|ToLoadingScreen
  (bind _returnvalue (Game|GetPlayerController 0))
  ;[1 1 1] Loading Screen
  (bind _returnvalue_2 (UserInterface|CreateWidget "/Game/Character/HUD/LoadingScreen_WBP.LoadingScreen_WBP_C" _returnvalue))
  (UserInterface|Viewport|AddtoPlayerScreen _returnvalue_2)
  (Variables|/Script/Engine.PlayerController|SetbShowMouseCursor _returnvalue true))

(event Custom|JoinSessionScreen
  (bind _returnvalue (Game|GetPlayerController 0))
  ;[1 1 1] Join Session Screen
  (bind _returnvalue_2 (UserInterface|CreateWidget "/Game/Character/HUD/JoinMenu_WBP.JoinMenu_WBP_C" _returnvalue))
  (UserInterface|Viewport|AddtoPlayerScreen _returnvalue_2)
  (Variables|/Script/Engine.PlayerController|SetbShowMouseCursor _returnvalue true))

(event Custom|HostServerScreen
  (bind _returnvalue (Game|GetPlayerController 0))
  ;[1 1 1] To Host Menu
  (bind _returnvalue_2 (UserInterface|CreateWidget "/Game/Character/HUD/HostMenu_WBP.HostMenu_WBP_C" _returnvalue))
  (UserInterface|Viewport|AddtoPlayerScreen _returnvalue_2)
  (Variables|/Script/Engine.PlayerController|SetbShowMouseCursor _returnvalue true))

(event Custom|CreateLobby
  (params (Number%20Of%20Players :type Integer) (ServerName :type Text) (Widget :type Widget%20Object%20Reference))
  ;[1 1 1] Create A Game Session
  (Variables|Default|SetNumberOfPlayers Number%20Of%20Players)
  (Variables|Default|SetServerName ServerName)
  (|Session (Game|GetPlayerController 0) 0 false
    (:OnSuccess
      (Utilities|LogtoScreen "Successfully created session")
      (Widget|RemovefromParent Widget)
      (CallFunction|ToLoadingScreen)
      (CallFunction|SpawnCharacter))
    (:OnFailure
      (Utilities|LogtoScreen "Couldn't create session"))))